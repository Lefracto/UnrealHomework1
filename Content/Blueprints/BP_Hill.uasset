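; BP_Hill is a health pickup that heals the third-person character and is consumed on use.
; It starts inactive on BeginPlay, and SetActive toggles the cube's collision and visibility along with the IsActive flag.
; While active, overlapping its collider with a BP_ThirdPersonCharacter adds HpToAdd health and destroys the actor.
; Nothing in this Blueprint activates it.
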(event `self.ReceiveBeginPlay`
  (`self.SetActive` false))

(event `self.Collider.OnComponentBeginOverlap`
  (params (OverlappedComponent :type "PrimitiveComponent Object Reference") (OtherActor :type "Actor Object Reference") (OtherComp :type "PrimitiveComponent Object Reference") (OtherBodyIndex :type Integer) (bFromSweep :type Boolean) (SweepResult :type "HitResult Structure (by ref)"))
  ;[1 1 1] Add hp on begin overlap and destroy object
  (if (`self.IsActive`)
    (bind _asbp_third_person_character (cast `/Game/ThirdPerson/Blueprints/BP_ThirdPersonCharacter` OtherActor))
    (`/Game/ThirdPerson/Blueprints/BP_ThirdPersonCharacter.AddHealth` _asbp_third_person_character (`self.HpToAdd`))
    (`self.K2_DestroyActor`)))

(fn `SetActive`
  (params (active :type Boolean))
  (bind _cube (`self.Cube`))
  (bind _cube_2 (`self.Cube`))
  (if active
    (`PrimitiveComponent.SetCollisionEnabled` _cube "QueryAndPhysics")
    (`SceneComponent.SetVisibility` _cube_2 true false)
    (set `self.IsActive` true)
    (else
      (`PrimitiveComponent.SetCollisionEnabled` _cube "NoCollision")
      (`SceneComponent.SetVisibility` _cube_2 false false)
      (set `self.IsActive` false))))

(fn `UserConstructionScript`)