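; BP_Room is a room actor built from child actors: four indexed doors, static and dynamic traps, hills and a hidden finish.
; BeginPlay activates the doors and makes a start room easy, while other functions look up or block doors by index.
; SetDifficulty colors the central light and calls GenerateTraps, which removes dynamic traps when easy, or activates a random hill and keeps one when hard.
; MakeFinish reveals the finish, recolors the light and destroys traps.
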(event `self.ReceiveBeginPlay`
  ;[1 1 1] Doors Initing
  (`self.Change Door Status` (`self.Door1`) true)
  (`self.Change Door Status` (`self.Door3`) true 2)
  (`self.Change Door Status` (`self.Door4`) true 3)
  (`self.Change Door Status` (`self.Door2`) true 1)
  ;[1 1 1] Finish Initing
  (`SceneComponent.SetVisibility` (`self.Finish`) false false)
  (if (`self.IsStart`)
    (`self.SetDifficulty` false)))

(fn `BlockAllDoors`
  (bind _asbp_door (cast `/Game/BP_Door` (`ChildActorComponent.ChildActor` (`self.Door4`))))
  (set `/Game/BP_Door.IsActiveDoor` false _asbp_door)
  (bind _asbp_door_2 (cast `/Game/BP_Door` (`ChildActorComponent.ChildActor` (`self.Door2`))))
  (set `/Game/BP_Door.IsActiveDoor` false _asbp_door_2)
  (bind _asbp_door_3 (cast `/Game/BP_Door` (`ChildActorComponent.ChildActor` (`self.Door3`))))
  (set `/Game/BP_Door.IsActiveDoor` false _asbp_door_3)
  (bind _asbp_door_4 (cast `/Game/BP_Door` (`ChildActorComponent.ChildActor` (`self.Door1`))))
  (set `/Game/BP_Door.IsActiveDoor` false _asbp_door_4))

(fn `BlockDoorsByIndexes`
  (params (DoorsToBlock :type "Array of Integer"))
  (for _array_element DoorsToBlock
    (bind _newparam (`self.GetDoorByIndex` _array_element))
    (set `/Game/BP_Door.IsActiveDoor` false _newparam)))

(fn `Change Door Status`
  (params (ChildActor :type "ChildActorComponent Object Reference") (IsActive :type Boolean) (DoorIndex :type Integer))
  ;[1 1 1] Make door active or not and give the index for it
  (bind _asbp_door (cast `/Game/BP_Door` (`ChildActorComponent.ChildActor` ChildActor)))
  (`/Game/BP_Door.SetActiveDoor` _asbp_door IsActive false)
  (set `/Game/BP_Door.DoorIndex` DoorIndex _asbp_door))

(fn `GenerateTraps`
  (locals (NewLocalVar :type "ChildActorComponent Object Reference"))
  (if (`self.Difficulty`)
    ;[1 1 1] Spawn(make visible) Hill in one of three spawn point for high difficulty
    (switch `int` (`KismetMathLibrary.RandomIntegerInRange` 0 2)
      (:`0`
        (set `self.HillToSpawn` (`self.Hill1`)))
      (:`1`
        (set `self.HillToSpawn` (`self.Hill3`)))
      (:`2`
        (set `self.HillToSpawn` (`self.Hill2`))))
    (bind _asbp_hill (cast `/Game/BP_Hill` (`ChildActorComponent.ChildActor` (`self.HillToSpawn`))))
    (`/Game/BP_Hill.SetActive` _asbp_hill true)
    ;[1 1 1] Delete one dynamic Traps of 2 for hard room
    (switch `int` (`KismetMathLibrary.RandomIntegerInRange` 0 1)
      (:`0`
        (`self.K2_DestroyActor` (`ChildActorComponent.ChildActor` (`self.BP_DynamicTrap_2`))))
      (:`1`
        (`self.K2_DestroyActor` (`ChildActorComponent.ChildActor` (`self.BP_DynamicTrap_1`)))))
    (else
      ;[1 1 1] Delete all dynamic traps for eay room
      (`self.K2_DestroyActor` (`ChildActorComponent.ChildActor` (`self.BP_DynamicTrap_1`)))
      (`self.K2_DestroyActor` (`ChildActorComponent.ChildActor` (`self.BP_DynamicTrap_2`))))))

(fn `GetDoorByIndex`
  (params (Index :type Integer))
  (returns (NewParam :type "/Game/BP_Door Object Reference"))
  ;[1 1 1] Just return door with given index
  (switch `int` Index
    (:`0`
      (bind _asbp_door (cast `/Game/BP_Door` (`ChildActorComponent.ChildActor` (`self.Door1`))))
      (return _asbp_door))
    (:`1`
      (bind _asbp_door_2 (cast `/Game/BP_Door` (`ChildActorComponent.ChildActor` (`self.Door2`))))
      (return _asbp_door_2))
    (:`2`
      (bind _asbp_door_3 (cast `/Game/BP_Door` (`ChildActorComponent.ChildActor` (`self.Door3`))))
      (return _asbp_door_3))
    (:`3`
      (bind _asbp_door_4 (cast `/Game/BP_Door` (`ChildActorComponent.ChildActor` (`self.Door4`))))
      (return _asbp_door_4))))

(fn `Make Finish`
  (bind _childactor (`ChildActorComponent.ChildActor` (`self.BP_DynamicTrap_1`)))
  (bind _childactor_2 (`ChildActorComponent.ChildActor` (`self.BP_DynamicTrap_2`)))
  ;[1 1 1] Make finish active and set color for room highlight
  (bind _asbp_finish (cast `/Game/BP_Finish` (`ChildActorComponent.ChildActor` (`self.Finish`))))
  (set `/Game/BP_Finish.IsActive` true _asbp_finish)
  (`SceneComponent.SetVisibility` (`self.Finish`) true false)
  (`LightComponent.SetLightColor` (`self.RoomDificultyLight`) (struct :`R` 1.0 :`G` 0.873234 :`A` 1.0) true)
  ;[1 1 1] Delete Traps for finish room
  (`self.K2_DestroyActor` (`ChildActorComponent.ChildActor` (`self.BP_StaticTrap_1`)))
  (`self.K2_DestroyActor` (`ChildActorComponent.ChildActor` (`self.BP_StaticTrap_2`)))
  (`/Engine/EditorBlueprintResources/StandardMacros.IsValid` _childactor
    (:`Is Valid`
      (`self.K2_DestroyActor` _childactor)
      (`/Engine/EditorBlueprintResources/StandardMacros.IsValid` _childactor_2
        (:`Is Valid`
          (`self.K2_DestroyActor` _childactor_2))))))

(fn `SetDifficulty`
  (params (Difficulty :type Boolean))
  (bind _roomdificultylight (`self.RoomDificultyLight`))
  ;[1 1 1] Set Color of Central Light and call Generate Trap
  (bind _output_get (set `self.Difficulty` Difficulty))
  (if _output_get
    (`LightComponent.SetLightColor` _roomdificultylight (struct :`R` 1.0 :`B` 0.017111 :`A` 1.0) true)
    (else
      (`LightComponent.SetLightColor` _roomdificultylight (struct :`G` 1.0 :`B` 0.069422 :`A` 1.0) true)))
  (`self.GenerateTraps`))

(fn `UserConstructionScript`)