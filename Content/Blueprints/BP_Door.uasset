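; BP_Door is a room door that requests the next room when the player walks into its trigger.
; An active door passes its DoorIndex to BP_SurvivalGameMode, hides itself, disables its trigger and tells its parent BP_Room to block all doors.
; An inactive door's trigger instead shows and solidifies the mesh, closing it once the player enters the new room.
; SetActiveDoor toggles mesh visibility, collision, active state and the trigger.
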(event `self.InCollider.OnComponentBeginOverlap`
  (params (OverlappedComponent :type "PrimitiveComponent Object Reference") (OtherActor :type "Actor Object Reference") (OtherComp :type "PrimitiveComponent Object Reference") (OtherBodyIndex :type Integer) (bFromSweep :type Boolean) (SweepResult :type "HitResult Structure (by ref)"))
  ;[1 1 1] Make open if player is on trigger || close all doors if one is closed || close yourself if player is in the new room
  (if (`self.IsActiveDoor`)
    (cast `/Game/ThirdPerson/Blueprints/BP_ThirdPersonCharacter` OtherActor)
    (bind _asbp_survival_game_modee (cast `/Game/ThirdPerson/Blueprints/BP_SurvivalGameMode` (`GameplayStatics.GetGameMode`)))
    (`/Game/ThirdPerson/Blueprints/BP_SurvivalGameMode.TryToGetNextRoom` _asbp_survival_game_modee (`self.DoorIndex`))
    (`self.SetActiveDoor` false true)
    (set `self.IsActiveDoor` false)
    (bind _asbp_room (cast `/Game/Blueprints/BP_Room` (`self.GetAttachParentActor`)))
    (`/Game/Blueprints/BP_Room.BlockAllDoors` _asbp_room)
    (else
      (cast `/Game/ThirdPerson/Blueprints/BP_ThirdPersonCharacter` OtherActor)
      (`SceneComponent.SetVisibility` (`self.StaticMesh`) true false)
      (`PrimitiveComponent.SetCollisionEnabled` (`self.StaticMesh`) "QueryAndPhysics"))))

(fn `SetActiveDoor`
  (params (isActive :type Boolean) (disableCollder :type Boolean))
  ;[1 1 1] Change collisions and visibility
  (`SceneComponent.SetVisibility` (`self.StaticMesh`) isActive false)
  (if isActive
    (`PrimitiveComponent.SetCollisionEnabled` (`self.StaticMesh`) "QueryAndPhysics")
    (set `self.IsActiveDoor` true)
    (else
      (`PrimitiveComponent.SetCollisionEnabled` (`self.StaticMesh`) "NoCollision")
      (set `self.IsActiveDoor` false)))
  (if disableCollder
    (`PrimitiveComponent.SetCollisionEnabled` (`self.InCollider`) "NoCollision")
    (else
      (`PrimitiveComponent.SetCollisionEnabled` (`self.InCollider`) "QueryAndPhysics"))))

(fn `UserConstructionScript`)