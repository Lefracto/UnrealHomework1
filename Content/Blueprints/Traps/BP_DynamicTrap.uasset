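; BP_DynamicTrap is a moving hazard that damages the third-person player character.
; On BeginPlay a looping timeline drives the static mesh along a spline by sampling its world location at the track's time value.
; When an actor overlap begins with a BP_ThirdPersonCharacter, it subtracts the Damage value from that character's health through AddHealth.
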(event `self.ReceiveBeginPlay`
  ;[1 1 1] Loop animation
  (bind (_direction _newtrack_0) (`Timeline|Timeline`)
    (:`Update`
      (`SceneComponent.K2_SetWorldLocation` (`self.StaticMesh`) (`SplineComponent.GetLocationAtTime` (`self.Spline`) _newtrack_0 "World" false) false false))
    (:`Finished`
      (`TimelineComponent.PlayFromStart` (`self.Timeline`)))))

(event `self.ReceiveActorBeginOverlap`
  (params (OtherActor :type "Actor Object Reference"))
  ;[1 1 1] Damage on overlaping
  (bind _asbp_third_person_character (cast `/Game/ThirdPerson/Blueprints/BP_ThirdPersonCharacter` OtherActor))
  (`/Game/ThirdPerson/Blueprints/BP_ThirdPersonCharacter.AddHealth` _asbp_third_person_character (* (`self.Damage`) -1.0)))

(fn `UserConstructionScript`)