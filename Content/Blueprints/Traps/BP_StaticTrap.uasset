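; BP_StaticTrap is a trap that drains the player's health while they stand inside its Box.
; Box overlap events cast to BP_ThirdPersonCharacter, storing the player and toggling the IsPlayerIn flag on enter and exit.
; Tick subtracts Damage through AddHealth every frame while the flag is set, so the damage rate depends on frame rate rather than delta time.
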(event `self.ReceiveTick`
  (params (DeltaSeconds :type "Float (single-precision)"))
  ;[1 1 1] Making damage
  (if (`self.IsPlayerIn`)
    (`/Game/ThirdPerson/Blueprints/BP_ThirdPersonCharacter.AddHealth` (`self.Player`) (* (`self.Damage`) -1.0))))

(event `self.Box.OnComponentBeginOverlap`
  (params (OverlappedComponent :type "PrimitiveComponent Object Reference") (OtherActor :type "Actor Object Reference") (OtherComp :type "PrimitiveComponent Object Reference") (OtherBodyIndex :type Integer) (bFromSweep :type Boolean) (SweepResult :type "HitResult Structure (by ref)"))
  ;[1 1 1] Remember player in the start of overlap
  (bind _asbp_third_person_character (cast `/Game/ThirdPerson/Blueprints/BP_ThirdPersonCharacter` OtherActor))
  (set `self.Player` _asbp_third_person_character)
  (set `self.IsPlayerIn` true))

(event `self.Box.OnComponentEndOverlap`
  (params (OverlappedComponent :type "PrimitiveComponent Object Reference") (OtherActor :type "Actor Object Reference") (OtherComp :type "PrimitiveComponent Object Reference") (OtherBodyIndex :type Integer))
  ;[1 1 1] Disable making damage for player
  (cast `/Game/ThirdPerson/Blueprints/BP_ThirdPersonCharacter` OtherActor)
  (set `self.IsPlayerIn` false))

(fn `UserConstructionScript`)